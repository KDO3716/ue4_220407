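; BP_Character is a player character Blueprint that handles walking, sprinting and jumping.
; MoveFoward and MoveRight axis inputs add movement along directions derived from control yaw only, scaled by a Speed variable.
; Left Shift sprints by switching Speed between full and half input scale instead of changing movement component settings, and the Jump action calls the built-in Jump.
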(event EventBeginPlay)

(event Collision|EventActorBeginOverlap
  (params (OtherActor :type Actor%20Object%20Reference)))

(event EventTick
  (params (DeltaSeconds :type Float%20%28single-precision%29)))

(event Input|ActionEvents|InputActionJump
  (params (Key :type Key%20Structure :default "None"))
  ;[1 1 1] 캐릭터 이동
  ;;[1 1 1] 점프
  (:Pressed
    (Character|Jump)))

(event Input|AxisEvents|InputAxisMoveFoward
  (params (AxisValue :type Float%20%28single-precision%29))
  ;[1 1 1] 캐릭터 이동
  (Pawn|Input|AddMovementInput (Math|Vector|GetForwardVector (Math|Rotator|MakeRotator 0.0 0.0 (.Yaw (Math|Rotator|BreakRotator (Pawn|GetControlRotation :!class /Script/Engine.Pawn))))) (* AxisValue (Variables|디폴트|Getspeed)) false))

(event Input|AxisEvents|InputAxisMoveRight
  (params (AxisValue :type Float%20%28single-precision%29))
  ;[1 1 1] 캐릭터 이동
  (Pawn|Input|AddMovementInput (Math|Vector|GetRightVector (Math|Rotator|MakeRotator 0.0 0.0 (.Yaw (Math|Rotator|BreakRotator (Pawn|GetControlRotation :!class /Script/Engine.Pawn))))) (* AxisValue (Variables|디폴트|Getspeed)) false))

(event Input|KeyboardEvents|LeftShift
  (params (Key :type Key%20Structure :default "None"))
  ;[1 1 1] 캐릭터 이동
  ;;[1 1 1] 달리기 속도 조절
  (:Pressed
    (Variables|디폴트|Setspeed 1.0))
  (:Released
    (Variables|디폴트|Setspeed 0.5)))

(fn ConstructionScript)